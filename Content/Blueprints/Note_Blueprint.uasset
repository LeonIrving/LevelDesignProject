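; Readable note pickup actor that shows a prompt on overlap and lets the player open and close a note with E.
; Overlap enables input and passes the note's Image index to FirstPersonCharacter; leaving disables input and removes both widgets.
; A FlipFlop toggles the note widget, playing a sound on opening and setting the character flag matching that index.
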(event Collision|EventActorBeginOverlap
  (params (OtherActor :type Actor%20Object%20Reference))
  (bind _returnvalue (UserInterface|CreateWidget "/Game/UI/PromptWidget.PromptWidget_C"))
  (UserInterface|Viewport|AddtoViewport _returnvalue 0)
  (Input|EnableInput (Game|GetPlayerController 0))
  (bind _asfirst_person_character (Utilities|Casting|CastToFirstPersonCharacter (Game|GetPlayerCharacter 0)))
  (Variables|/Game/FirstPersonBP/Blueprints/FirstPersonCharacter.FirstPersonCharacter_C|SetImageIndex _asfirst_person_character (Variables|Default|GetImage)))

(event Collision|EventActorEndOverlap
  (params (OtherActor :type Actor%20Object%20Reference))
  (Widget|RemovefromParent (stale Collision|EventActorBeginOverlap _returnvalue))
  (Input|DisableInput 0)
  (Widget|RemovefromParent (stale Input|KeyboardEvents|E _returnvalue)))

(event Input|KeyboardEvents|E
  (params (Key :type Key%20Structure))
  (:Pressed
    (Utilities|FlowControl|FlipFlop
      (:A
        (bind _returnvalue (UserInterface|CreateWidget "/Game/UI/NoteWidget.NoteWidget_C"))
        (UserInterface|Viewport|AddtoViewport _returnvalue 0)
        (Audio|PlaySound2D "/Game/Audio/SoundEffects/SND_Open_Letter.SND_Open_Letter")
        (bind _asfirst_person_character (Utilities|Casting|CastToFirstPersonCharacter (Game|GetPlayerCharacter 0)))
        (if (== (Variables|Default|GetImage) 0)
          (Variables|/Game/FirstPersonBP/Blueprints/FirstPersonCharacter.FirstPersonCharacter_C|SetHasNote1 _asfirst_person_character true)
          (elif (== (Variables|Default|GetImage) 1)
            (Variables|/Game/FirstPersonBP/Blueprints/FirstPersonCharacter.FirstPersonCharacter_C|SetHasNote2 _asfirst_person_character true)
            (elif (== (Variables|Default|GetImage) 2)
              (Variables|/Game/FirstPersonBP/Blueprints/FirstPersonCharacter.FirstPersonCharacter_C|SetHas1 _asfirst_person_character true)))))
      (:B
        (Widget|RemovefromParent _returnvalue)))))

(fn ConstructionScript)